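; BP_Flame is a fire effect actor that turns to face the first player's pawn and tints its flame.
; Each tick, its Sphere component interpolates toward a look-at rotation with a fixed 90-degree corrective offset, at a speed set by InterpSpeed.
; Tick also reapplies the R, G, B, A variables to FlameFx's Color parameter and prints both sphere and player locations for debugging.
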(event EventBeginPlay)

(event EventTick
  (params (DeltaSeconds :type Float%20%28single-precision%29))
  (bind _returnvalue (Game|Player|GetPlayerPawn 0))
  (bind _sphere (Variables|Default|GetSphere))
  (bind _returnvalue_2 (Transformation|GetWorldLocation _sphere))
  (bind _returnvalue_3 (Transformation|GetActorLocation _returnvalue))
  (bind _returnvalue_4 (Math|Rotator|FindLookatRotation _returnvalue_2 _returnvalue_3))
  (Development|PrintString (Utilities|String|Append (Utilities|String|ToString(Vector) _returnvalue_2) " / " (Utilities|String|ToString(Vector) _returnvalue_3)))
  (Transformation|SetWorldRotation (Variables|Default|GetSphere) (Math|Interpolation|RInterpTo (Transformation|GetWorldRotation (Variables|Default|GetSphere)) (Math|Rotator|CombineRotators (Math|Rotator|MakeRotator (.roll _returnvalue_4) (.pitch _returnvalue_4) (.yaw _returnvalue_4)) "0.000000,-90.000000,0.000000") DeltaSeconds (Variables|Default|GetInterp%20Speed)) false false)
  (Effects|Components|ParticleSystem|SetColorParameter (Variables|Default|GetFlameFx) "Color" (Math|Color|MakeColor (Variables|Default|GetR) (Variables|Default|GetG) (Variables|Default|GetB) (Variables|Default|GetA))))

(fn ConstructionScript)